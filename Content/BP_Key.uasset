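; BP_Key is a pickup actor that, on Interact, adds its key ID to the player's BP_ThirdPersonCharacter, destroys itself and prints "Door Unlocked".
; A box overlap shows its TextRender while that character is inside and hides it on exit.
; Each tick, the text turns on yaw only to face the player camera.
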(event OnComponentBeginOverlap(Box)
  (params (OverlappedComponent :type Primitive%20Component%20Object%20Reference) (OtherActor :type Actor%20Object%20Reference) (OtherComp :type Primitive%20Component%20Object%20Reference) (OtherBodyIndex :type Integer) (bFromSweep :type Boolean) (SweepResult :type Hit%20Result%20Structure%20%28by%20ref%29))
  ;[0.2031 0.2031 0.2031] Text Visibility Toggle
  (Utilities|Casting|CastToBP_ThirdPersonCharacter OtherActor)
  (Development|SetHiddeninGame (Variables|Default|GetText%20Render) false false))

(event OnComponentEndOverlap(Box)
  (params (OverlappedComponent :type Primitive%20Component%20Object%20Reference) (OtherActor :type Actor%20Object%20Reference) (OtherComp :type Primitive%20Component%20Object%20Reference) (OtherBodyIndex :type Integer))
  ;[0.2031 0.2031 0.2031] Text Visibility Toggle
  (Utilities|Casting|CastToBP_ThirdPersonCharacter OtherActor)
  (Development|SetHiddeninGame (Variables|Default|GetText%20Render) true false))

(event EventBeginPlay)

(event EventTick
  (params (DeltaSeconds :type Float%20%28single-precision%29))
  ;[0.2031 0.2031 0.2031] Text Face Player
  (Transformation|SetWorldRotation (Variables|Default|GetText%20Render) (Math|Rotator|MakeRotator 0.0 0.0 (.yaw (Math|Rotator|FindLookatRotation (Transformation|GetActorLocation) (Transformation|GetActorLocation (Game|GetPlayerCameraManager 0))))) false false))

(event EventInteract
  ;[0.2031 0.2031 0.2031] Interactivity
  (bind _asbp_third_person_character (Utilities|Casting|CastToBP_ThirdPersonCharacter (Game|GetPlayerCharacter 0)))
  (Default|AddKey _asbp_third_person_character (Variables|/Game/KeyComponent.KeyComponent_C|GetID (Variables|Default|GetKey)))
  (Actor|DestroyActor)
  (Development|PrintText "Door Unlocked"))

(fn ConstructionScript)